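; BP_HandVR is a VR hand Blueprint that casts a debug line trace from its hand mesh while the left motion controller trigger is held.
; The trigger's press and release toggle a LineTracing flag.
; Tick checks that flag and traces forward on the Visibility channel, drawing the line for a duration.
; The hit result is not used.
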(event `Key|MotionController_Left_Trigger`
  (params (Key :type "Key Structure"))
  (:`Pressed`
    (set `self.LineTracing` true))
  (:`Released`
    (set `self.LineTracing` false)))

(event `self.ReceiveTick`
  (params (DeltaSeconds :type "Float (single-precision)"))
  (bind _handmesh (`self.HandMesh`))
  (bind _returnvalue (`SceneComponent.K2_GetComponentLocation` _handmesh))
  (if (`self.LineTracing`)
    (`KismetSystemLibrary.LineTraceSingle` :`Start` _returnvalue :`End` (+ _returnvalue (* (`SceneComponent.GetForwardVector` _handmesh) 10000.0)) :`TraceChannel` "TraceTypeQuery1" :`DrawDebugType` "ForDuration")))

(fn `UserConstructionScript`)